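; AI controller for PvE enemies that switches between patrolling and chasing the player, without a behavior tree.
; AI Perception sets a CanSeePlayer flag for player pawn 0, stops movement and starts chase or patrol; possession starts both loops after a delay.
; Chase and patrol are self-recalling AIMoveTo loops gated by that flag.
; Patrol cycles through BP_EnemyAI_Test's patrol points, advancing even after failed moves, while a failed chase only prints.
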(event OnTargetPerceptionUpdated(AIPerception)
  (params (Actor :type Actor%20Object%20Reference) (Stimulus :type AI%20Stimulus%20Structure))
  (if (and (== Actor (Game|Player|GetPlayerPawn 0)) (.bSuccessfullySensed (Utilities|Struct|BreakAIStimulus Stimulus)))
    (Variables|Default|SetCanSeePlayer true)
    (AI|Navigation|StopMovement)
    (CallFunction|UpdateChase)
    (else
      (Variables|Default|SetCanSeePlayer false)
      (AI|Navigation|StopMovement)
      (CallFunction|UpdatePatrol))))

(event Custom|UpdateChase
  (bind _returnvalue (Game|Player|GetPlayerPawn 0))
  (Utilities|IsValid _returnvalue
    (:Is%20Valid
      (if (Variables|Default|GetCanSeePlayer)
        (AI|AIMoveTo (stale EventPossess PossessedPawn) "0, 0, 0" _returnvalue 1e+02 false
          (:OnSuccess
            (Utilities|FlowControl|Delay 0.5)
            (CallFunction|UpdateChase))
          (:OnFail
            (Development|PrintString "AI MOVE FAILED" false)))))
    (:Is%20Not%20Valid
      (Development|PrintString "PLAYER IS NOT FOUND"))))

(event Custom|UpdatePatrol
  (bind _returnvalue (Pawn|GetControlledPawn))
  (bind _asbp_enemy_ai_test (Utilities|Casting|CastToBP_EnemyAI_Test _returnvalue))
  (if (> (Utilities|Array|Length (Variables|/Game/Estival/AddGameModes/PvE/BP_EnemyAI_Test.BP_EnemyAI_Test_C|GetPatrolPoints _asbp_enemy_ai_test)) 0)
    (if (not (Variables|Default|GetCanSeePlayer))
      (if (Utilities|Array|IsValidIndex (Variables|/Game/Estival/AddGameModes/PvE/BP_EnemyAI_Test.BP_EnemyAI_Test_C|GetPatrolPoints _asbp_enemy_ai_test) (Variables|/Game/Estival/AddGameModes/PvE/BP_EnemyAI_Test.BP_EnemyAI_Test_C|GetPatrolIndex _asbp_enemy_ai_test))
        (Development|PrintString (Utilities|String|ToString(Integer) (Variables|/Game/Estival/AddGameModes/PvE/BP_EnemyAI_Test.BP_EnemyAI_Test_C|GetPatrolIndex _asbp_enemy_ai_test)))
        (AI|AIMoveTo _returnvalue "0, 0, 0" (Utilities|Array|Get(acopy) (Variables|/Game/Estival/AddGameModes/PvE/BP_EnemyAI_Test.BP_EnemyAI_Test_C|GetPatrolPoints _asbp_enemy_ai_test) (Variables|/Game/Estival/AddGameModes/PvE/BP_EnemyAI_Test.BP_EnemyAI_Test_C|GetPatrolIndex _asbp_enemy_ai_test)) 5.0 false
          (:OnSuccess
            (Utilities|FlowControl|Delay 1.0 :!label _label)
            (if (not (Variables|Default|GetCanSeePlayer))
              (Variables|/Game/Estival/AddGameModes/PvE/BP_EnemyAI_Test.BP_EnemyAI_Test_C|SetPatrolIndex _asbp_enemy_ai_test (Math|Integer|%(Integer) (+ (Variables|/Game/Estival/AddGameModes/PvE/BP_EnemyAI_Test.BP_EnemyAI_Test_C|GetPatrolIndex _asbp_enemy_ai_test) 1) (Utilities|Array|Length (Variables|/Game/Estival/AddGameModes/PvE/BP_EnemyAI_Test.BP_EnemyAI_Test_C|GetPatrolPoints _asbp_enemy_ai_test))))
              (CallFunction|UpdatePatrol)))
          (:OnFail
            (Development|PrintString "PATROL MOVE FAILED" false)
            (if (not (Variables|Default|GetCanSeePlayer))
              (goto _label))))))))

(event EventBeginPlay)

(event EventTick
  (params (DeltaSeconds :type Float%20%28single-precision%29)))

(event EventPossess
  (params (PossessedPawn :type Pawn%20Object%20Reference))
  (Utilities|FlowControl|Sequence
    (:then_0
      (Utilities|FlowControl|Delay 1.0)
      (CallFunction|UpdateChase))
    (:then_1
      (Utilities|FlowControl|Delay 1.0)
      (CallFunction|UpdatePatrol))))

(fn ConstructionScript)