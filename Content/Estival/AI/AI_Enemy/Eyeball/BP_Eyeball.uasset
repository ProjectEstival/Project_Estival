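; Eyeball enemy Blueprint that flashes when it takes non-lethal damage.
; It listens for resource changes and reacts only when Health drops while staying above zero.
; The mesh gets a hit-flash overlay material, which a short retriggerable delay clears, so rapid hits extend the flash instead of stacking.
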(event OnResourceChanged(Resources)
  (params (Stat :type Gameplay%20Tag%20Structure) (NewValue :type Float%20%28single-precision%29) (OldValue :type Float%20%28single-precision%29) (MaxValue :type Float%20%28single-precision%29))
  (if (== Stat "(TagName=\"Stats.Resources.Health\")")
    (if (and (< NewValue OldValue) (> NewValue 0.0))
      (Rendering|Material|SetOverlayMaterial (Variables|Character|GetMesh) "/Game/Estival/AI/AI_Enemy/Eyeball/Materials/M_EyeballHitFlash.M_EyeballHitFlash" false 0 :!class /Script/Engine.MeshComponent)
      (Utilities|FlowControl|RetriggerableDelay 0.1)
      (Rendering|Material|SetOverlayMaterial (Variables|Character|GetMesh) 0 false 0 :!class /Script/Engine.MeshComponent))))

(fn ConstructionScript)