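; BP_Blockout_Hammer is a test character Blueprint for previewing animation montages from the keyboard.
; Number pad keys one through nine each pass their matching Animation variable to a shared Play Montage graph.
; That graph checks the montage is valid, then plays it on the character at normal rate, so empty slots do nothing.
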(event Input|KeyboardEvents|NumPadThree
  (params (Key :type Key%20Structure :default "None"))
  (:Pressed
    (Utilities|PlayMontage (Variables|Animation|GetAnimation%203))))

(event Input|KeyboardEvents|NumPadNine
  (params (Key :type Key%20Structure :default "None"))
  (:Pressed
    (Utilities|PlayMontage (Variables|Animation|GetAnimation%209))))

(event Input|KeyboardEvents|NumPadTwo
  (params (Key :type Key%20Structure :default "None"))
  (:Pressed
    (Utilities|PlayMontage (Variables|Animation|GetAnimation%202))))

(event Input|KeyboardEvents|NumPadFour
  (params (Key :type Key%20Structure :default "None"))
  (:Pressed
    (Utilities|PlayMontage (Variables|Animation|GetAnimation%204))))

(event Input|KeyboardEvents|NumPadFive
  (params (Key :type Key%20Structure :default "None"))
  (:Pressed
    (Utilities|PlayMontage (Variables|Animation|GetAnimation%205))))

(event Input|KeyboardEvents|NumPadOne
  (params (Key :type Key%20Structure :default "None"))
  (:Pressed
    (Utilities|PlayMontage (Variables|Animation|GetAnimation%201))))

(event Input|KeyboardEvents|NumPadSix
  (params (Key :type Key%20Structure :default "None"))
  (:Pressed
    (Utilities|PlayMontage (Variables|Animation|GetAnimation%206))))

(event Input|KeyboardEvents|NumPadSeven
  (params (Key :type Key%20Structure :default "None"))
  (:Pressed
    (Utilities|PlayMontage (Variables|Animation|GetAnimation%207))))

(event Input|KeyboardEvents|NumPadEight
  (params (Key :type Key%20Structure :default "None"))
  (:Pressed
    (Utilities|PlayMontage (Variables|Animation|GetAnimation%208))))

(fn ConstructionScript
  (|CallParentFunction))